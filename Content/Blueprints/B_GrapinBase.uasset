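; B_GrapinBase is an actor, apparently a grappling-hook base by its name, that follows the player character and orients itself against their movement.
; Every Tick it moves to player 0's location without sweeping.
; When the capsule's physics linear velocity exceeds a small threshold, it sets its rotation by combining MakeRotFromX, Y and Z rotators, each built from the negated normalized velocity.
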(event EventBeginPlay)

(event Collision|EventActorBeginOverlap
  (params (OtherActor :type Actor%20Object%20Reference)))

(event EventTick
  (params (DeltaSeconds :type Float%20%28single-precision%29))
  (bind _returnvalue (Game|GetPlayerCharacter 0))
  (Transformation|SetActorLocation (Transformation|GetActorLocation _returnvalue) false false)
  (bind _returnvalue_2 (Physics|GetPhysicsLinearVelocity (Variables|/Script/Engine.Character|GetCapsuleComponent _returnvalue) "None"))
  (if (> (Math|Vector|VectorLength _returnvalue_2) 1e+01)
    (Transformation|SetActorRotation (Math|Rotator|CombineRotators (Math|Rotator|CombineRotators (Math|Rotator|MakeRotfromX (Math|Vector|MakeVector (* (.x (Math|Vector|Normalize _returnvalue_2)) -1.0) (* (.y (Math|Vector|Normalize _returnvalue_2)) -1.0) (* (.z (Math|Vector|Normalize _returnvalue_2)) -1.0))) (Math|Rotator|MakeRotfromY (Math|Vector|MakeVector (* (.x (Math|Vector|Normalize _returnvalue_2)) -1.0) (* (.y (Math|Vector|Normalize _returnvalue_2)) -1.0) (* (.z (Math|Vector|Normalize _returnvalue_2)) -1.0)))) (Math|Rotator|MakeRotfromZ (Math|Vector|MakeVector (* (.x (Math|Vector|Normalize _returnvalue_2)) -1.0) (* (.y (Math|Vector|Normalize _returnvalue_2)) -1.0) (* (.z (Math|Vector|Normalize _returnvalue_2)) -1.0)))))))

(fn ConstructionScript)