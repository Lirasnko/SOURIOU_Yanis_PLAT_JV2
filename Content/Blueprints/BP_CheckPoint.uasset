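; BP_CheckPoint is a checkpoint plate that becomes the player's active checkpoint when touched.
; Overlapping its box with a BP_ThirdPersonCharacter stores the checkpoint on that character.
; The character's previous checkpoint plate reverts to the inactive material, while this plate switches to the active material and spawns a Niagara activation effect at its location.
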(event OnComponentBeginOverlap(Box)
  (params (OverlappedComponent :type Primitive%20Component%20Object%20Reference) (OtherActor :type Actor%20Object%20Reference) (OtherComp :type Primitive%20Component%20Object%20Reference) (OtherBodyIndex :type Integer) (bFromSweep :type Boolean) (SweepResult :type Hit%20Result%20Structure%20%28by%20ref%29))
  (bind _asbp_third_person_character (Utilities|Casting|CastToBP_ThirdPersonCharacter OtherActor))
  (if (Utilities|IsValid (Variables|/Game/ThirdPerson/Blueprints/BP_ThirdPersonCharacter.BP_ThirdPersonCharacter_C|GetCheckPoint _asbp_third_person_character))
    (Rendering|Material|SetMaterial (Variables|BP_CheckPoint_C|GetPlate (Variables|/Game/ThirdPerson/Blueprints/BP_ThirdPersonCharacter.BP_ThirdPersonCharacter_C|GetCheckPoint _asbp_third_person_character)) 0 "/Game/Materials/Spawner_Plate/MI_SpawnerPlate_Player.MI_SpawnerPlate_Player"))
  (Variables|/Game/ThirdPerson/Blueprints/BP_ThirdPersonCharacter.BP_ThirdPersonCharacter_C|SetCheckPoint _asbp_third_person_character self)
  (Rendering|Material|SetMaterial (Variables|Default|GetPlate) 0 "/Game/Materials/Spawner_Plate/MI_SpawnerPlate_Player_Active.MI_SpawnerPlate_Player_Active")
  (Niagara|SpawnSystematLocation "/Game/Particles/NPS_ActiveCheckPoint.NPS_ActiveCheckPoint" (Transformation|GetActorLocation) "0, 0, 0" "1.100000,1.100000,1.100000"))

(event EventBeginPlay)

(event Collision|EventActorBeginOverlap
  (params (OtherActor :type Actor%20Object%20Reference)))

(event EventTick
  (params (DeltaSeconds :type Float%20%28single-precision%29)))

(fn ConstructionScript)