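; Base item actor that idles with a spinning, bobbing mesh and can fly to the player when MoveTo is called.
; A looping timeline alternates play and reverse to bob the mesh, while Tick adds a fixed, frame-rate-dependent rotation.
; MoveTo runs a second timeline that lerps the actor toward the player's live location, blocking new bob cycles until it finishes.
; No pickup or overlap logic is implemented here.
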(event Custom|Move
  (if (not (Variables|Default|GetMoving))
    (if (Variables|Default|GetDown)
      (bind _newtrack_0 (Timeline|Timeline Play)
        (:Update
          (Transformation|SetRelativeLocation (Variables|Default|GetStaticMesh) (Math|Vector|Lerp(Vector) "0, 0, 0" "0.000000,0.000000,-30.000000" _newtrack_0) false false))
        (:Finished
          (if (Variables|Default|GetDown)
            (Variables|Default|SetDown false)
            (else
              (Variables|Default|SetDown true)))
          (CallFunction|Move)))
      (else
        (Timeline|Timeline Reverse)))))

(event Custom|MoveTo
  (Variables|Default|SetMoving true)
  (Variables|Default|SetStartPos (Transformation|GetActorLocation))
  (bind _newtrack_0 (Timeline|Movement Play)
    (:Update
      (Transformation|SetActorLocation (Math|Vector|Lerp(Vector) (Variables|Default|GetStartPos) (Transformation|GetActorLocation (Game|GetPlayerCharacter 0)) _newtrack_0) false false))
    (:Finished
      (Variables|Default|SetMoving false)
      (CallFunction|Move))))

(event EventBeginPlay
  (Components|Timeline|SetPlayRate (Variables|Default|GetMovement) 3.0)
  (Components|Timeline|SetPlayRate (Variables|Default|GetTimeline) 0.5)
  (CallFunction|Move))

(event Collision|EventActorBeginOverlap
  (params (OtherActor :type Actor%20Object%20Reference)))

(event EventTick
  (params (DeltaSeconds :type Float%20%28single-precision%29))
  (bind _staticmesh (Variables|Default|GetStaticMesh))
  (Transformation|SetRelativeRotation _staticmesh (Math|Rotator|CombineRotators (Variables|/Script/Engine.SceneComponent|GetRelativeRotation _staticmesh) "0.000000,2.000000,0.000000") false false))

(fn ConstructionScript)