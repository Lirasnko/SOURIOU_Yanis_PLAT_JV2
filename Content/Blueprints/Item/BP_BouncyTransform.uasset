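; BP_BouncyTransform is a pickup item that turns a sticky third-person character bouncy.
; A sphere overlap casts to BP_ThirdPersonCharacter and only proceeds if that character is Sticky.
; It plays the character's smoke, disables GrabSphere collision, then after a short delay calls SetBouncy and the health change visual.
; Finally it clears its Spawner's Item reference and destroys itself.
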(event OnComponentBeginOverlap(Sphere)
  (params (OverlappedComponent :type Primitive%20Component%20Object%20Reference) (OtherActor :type Actor%20Object%20Reference) (OtherComp :type Primitive%20Component%20Object%20Reference) (OtherBodyIndex :type Integer) (bFromSweep :type Boolean) (SweepResult :type Hit%20Result%20Structure%20%28by%20ref%29))
  (bind _asbp_third_person_character (Utilities|Casting|CastToBP_ThirdPersonCharacter OtherActor))
  (if (Variables|/Game/ThirdPerson/Blueprints/BP_ThirdPersonCharacter.BP_ThirdPersonCharacter_C|Getsticky _asbp_third_person_character)
    (Default|Smoke _asbp_third_person_character)
    (Collision|SetCollisionEnabled (Variables|Default|GetGrabSphere) "NoCollision")
    (Utilities|FlowControl|Delay 0.15)
    (Default|SetBouncy _asbp_third_person_character)
    (Default|HealthModificationVisual _asbp_third_person_character)
    (Variables|/Game/Blueprints/Spawner/BP_Spawner.BP_Spawner_C|SetItem (Variables|Default|GetSpawner) 0)
    (Actor|DestroyActor)))

(event EventBeginPlay
  (|CallParentFunction) ; This node is disabled and will not be called.\nDrag off pins to build functionality.
)

(event Collision|EventActorBeginOverlap
  (params (OtherActor :type Actor%20Object%20Reference))
  (|CallParentFunction OtherActor) ; This node is disabled and will not be called.\nDrag off pins to build functionality.
)

(event EventTick
  (params (DeltaSeconds :type Float%20%28single-precision%29))
  (|CallParentFunction DeltaSeconds) ; This node is disabled and will not be called.\nDrag off pins to build functionality.
)

(fn ConstructionScript
  (|CallParentFunction))