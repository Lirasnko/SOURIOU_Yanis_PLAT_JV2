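; Grapple ("Grapin") base actor that follows the player character, registering itself as that character's GrapinObject on BeginPlay.
; Each tick it snaps to the player's location and, above a small speed threshold, tilts and yaws from the capsule's physics velocity.
; The rotation uses per-quadrant arccos/arcsin branches, with tilt scaled to a third.
; A Light event sets color and intensity parameters on the mesh's materials.
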(event Custom|Light
  (params (Color :type Linear%20Color%20Structure) (Intensity :type Float%20%28single-precision%29))
  (Rendering|Material|SetColorParameterValueonMaterials (Variables|Default|GetStaticMesh) "LightColor" Color)
  (Rendering|Material|SetScalarParameterValueonMaterials (Variables|Default|GetStaticMesh) "Intensity" Intensity))

(event EventBeginPlay
  (bind _returnvalue (Rendering|Material|CreateDynamicMaterialInstance "/Game/Materials/Items/MI_GrapinBase.MI_GrapinBase" "None" "None" :!class /Script/Engine.KismetMaterialLibrary))
  (Variables|Default|SetMaterialInstance _returnvalue)
  (bind _returnvalue_2 (Actor|GetActorOfClass "/Game/ThirdPerson/Blueprints/BP_ThirdPersonCharacter.BP_ThirdPersonCharacter_C"))
  (Variables|/Game/ThirdPerson/Blueprints/BP_ThirdPersonCharacter.BP_ThirdPersonCharacter_C|SetGrapinObject _returnvalue_2 self))

(event Collision|EventActorBeginOverlap
  (params (OtherActor :type Actor%20Object%20Reference)))

(event EventTick
  (params (DeltaSeconds :type Float%20%28single-precision%29))
  (bind _returnvalue (Game|GetPlayerCharacter 0))
  (Transformation|SetActorLocation (Transformation|GetActorLocation _returnvalue) false false)
  (bind _returnvalue_2 (Physics|GetPhysicsLinearVelocity (Variables|/Script/Engine.Character|GetCapsuleComponent _returnvalue) "None"))
  (if (> (Math|Vector|VectorLength _returnvalue_2) 1e+01)
    (if (> (Class|KismetMathLibrary|DegAcos (* (.z (Math|Vector|Normalize (Math|Vector|MakeVector (.X (Math|Vector|BreakVector _returnvalue_2)) (.Y (Math|Vector|BreakVector _returnvalue_2)) (.Z (Math|Vector|BreakVector _returnvalue_2))))) -1.0)) 9e+01)
      (if (> (* (.x (Math|Vector|Normalize (Math|Vector|MakeVector (.X (Math|Vector|BreakVector _returnvalue_2)) (.Y (Math|Vector|BreakVector _returnvalue_2)) 0.0))) -1.0) 0.0)
        (if (> (* (.y (Math|Vector|Normalize (Math|Vector|MakeVector (.X (Math|Vector|BreakVector _returnvalue_2)) (.Y (Math|Vector|BreakVector _returnvalue_2)) 0.0))) -1.0) 0.0)
          (Transformation|SetActorRotation (Math|Rotator|MakeRotator (/ (+ (* (Class|KismetMathLibrary|DegAcos (* (.z (Math|Vector|Normalize (Math|Vector|MakeVector (.X (Math|Vector|BreakVector _returnvalue_2)) (.Y (Math|Vector|BreakVector _returnvalue_2)) (.Z (Math|Vector|BreakVector _returnvalue_2))))) -1.0)) -1.0) 1.8e+02) 3.0) 0.0 (+ (Class|KismetMathLibrary|DegAsin (* (.y (Math|Vector|Normalize (Math|Vector|MakeVector (.X (Math|Vector|BreakVector _returnvalue_2)) (.Y (Math|Vector|BreakVector _returnvalue_2)) 0.0))) -1.0)) -9e+01)))
          (else
            (Transformation|SetActorRotation (Math|Rotator|MakeRotator (/ (+ (* (Class|KismetMathLibrary|DegAcos (* (.z (Math|Vector|Normalize (Math|Vector|MakeVector (.X (Math|Vector|BreakVector _returnvalue_2)) (.Y (Math|Vector|BreakVector _returnvalue_2)) (.Z (Math|Vector|BreakVector _returnvalue_2))))) -1.0)) -1.0) 1.8e+02) 3.0) 0.0 (+ (Class|KismetMathLibrary|DegAsin (* (.y (Math|Vector|Normalize (Math|Vector|MakeVector (.X (Math|Vector|BreakVector _returnvalue_2)) (.Y (Math|Vector|BreakVector _returnvalue_2)) 0.0))) -1.0)) 2.7e+02)))))
        (elif (> (* (.y (Math|Vector|Normalize (Math|Vector|MakeVector (.X (Math|Vector|BreakVector _returnvalue_2)) (.Y (Math|Vector|BreakVector _returnvalue_2)) 0.0))) -1.0) 0.0)
          (Transformation|SetActorRotation (Math|Rotator|MakeRotator (/ (+ (* (Class|KismetMathLibrary|DegAcos (* (.z (Math|Vector|Normalize (Math|Vector|MakeVector (.X (Math|Vector|BreakVector _returnvalue_2)) (.Y (Math|Vector|BreakVector _returnvalue_2)) (.Z (Math|Vector|BreakVector _returnvalue_2))))) -1.0)) -1.0) 1.8e+02) 3.0) 0.0 (+ (Class|KismetMathLibrary|DegAcos (* (.x (Math|Vector|Normalize (Math|Vector|MakeVector (.X (Math|Vector|BreakVector _returnvalue_2)) (.Y (Math|Vector|BreakVector _returnvalue_2)) 0.0))) -1.0)) -9e+01)))
          (else
            (Transformation|SetActorRotation (Math|Rotator|MakeRotator (/ (+ (* (Class|KismetMathLibrary|DegAcos (* (.z (Math|Vector|Normalize (Math|Vector|MakeVector (.X (Math|Vector|BreakVector _returnvalue_2)) (.Y (Math|Vector|BreakVector _returnvalue_2)) (.Z (Math|Vector|BreakVector _returnvalue_2))))) -1.0)) -1.0) 1.8e+02) 3.0) 0.0 (+ (* (Class|KismetMathLibrary|DegAcos (* (.x (Math|Vector|Normalize (Math|Vector|MakeVector (.X (Math|Vector|BreakVector _returnvalue_2)) (.Y (Math|Vector|BreakVector _returnvalue_2)) 0.0))) -1.0)) -1.0) 2.7e+02))))))
      (elif (> (* (.x (Math|Vector|Normalize (Math|Vector|MakeVector (.X (Math|Vector|BreakVector _returnvalue_2)) (.Y (Math|Vector|BreakVector _returnvalue_2)) 0.0))) -1.0) 0.0)
        (if (> (* (.y (Math|Vector|Normalize (Math|Vector|MakeVector (.X (Math|Vector|BreakVector _returnvalue_2)) (.Y (Math|Vector|BreakVector _returnvalue_2)) 0.0))) -1.0) 0.0)
          (Transformation|SetActorRotation (Math|Rotator|MakeRotator (/ (Class|KismetMathLibrary|DegAcos (* (.z (Math|Vector|Normalize (Math|Vector|MakeVector (.X (Math|Vector|BreakVector _returnvalue_2)) (.Y (Math|Vector|BreakVector _returnvalue_2)) (.Z (Math|Vector|BreakVector _returnvalue_2))))) -1.0)) 3.0) 0.0 (+ (Class|KismetMathLibrary|DegAsin (* (.y (Math|Vector|Normalize (Math|Vector|MakeVector (.X (Math|Vector|BreakVector _returnvalue_2)) (.Y (Math|Vector|BreakVector _returnvalue_2)) 0.0))) -1.0)) -9e+01)))
          (else
            (Transformation|SetActorRotation (Math|Rotator|MakeRotator (/ (Class|KismetMathLibrary|DegAcos (* (.z (Math|Vector|Normalize (Math|Vector|MakeVector (.X (Math|Vector|BreakVector _returnvalue_2)) (.Y (Math|Vector|BreakVector _returnvalue_2)) (.Z (Math|Vector|BreakVector _returnvalue_2))))) -1.0)) 3.0) 0.0 (+ (Class|KismetMathLibrary|DegAsin (* (.y (Math|Vector|Normalize (Math|Vector|MakeVector (.X (Math|Vector|BreakVector _returnvalue_2)) (.Y (Math|Vector|BreakVector _returnvalue_2)) 0.0))) -1.0)) 2.7e+02)))))
        (elif (> (* (.y (Math|Vector|Normalize (Math|Vector|MakeVector (.X (Math|Vector|BreakVector _returnvalue_2)) (.Y (Math|Vector|BreakVector _returnvalue_2)) 0.0))) -1.0) 0.0)
          (Transformation|SetActorRotation (Math|Rotator|MakeRotator (/ (Class|KismetMathLibrary|DegAcos (* (.z (Math|Vector|Normalize (Math|Vector|MakeVector (.X (Math|Vector|BreakVector _returnvalue_2)) (.Y (Math|Vector|BreakVector _returnvalue_2)) (.Z (Math|Vector|BreakVector _returnvalue_2))))) -1.0)) 3.0) 0.0 (+ (Class|KismetMathLibrary|DegAcos (* (.x (Math|Vector|Normalize (Math|Vector|MakeVector (.X (Math|Vector|BreakVector _returnvalue_2)) (.Y (Math|Vector|BreakVector _returnvalue_2)) 0.0))) -1.0)) -9e+01)))
          (else
            (Transformation|SetActorRotation (Math|Rotator|MakeRotator (/ (Class|KismetMathLibrary|DegAcos (* (.z (Math|Vector|Normalize (Math|Vector|MakeVector (.X (Math|Vector|BreakVector _returnvalue_2)) (.Y (Math|Vector|BreakVector _returnvalue_2)) (.Z (Math|Vector|BreakVector _returnvalue_2))))) -1.0)) 3.0) 0.0 (+ (* (Class|KismetMathLibrary|DegAcos (* (.x (Math|Vector|Normalize (Math|Vector|MakeVector (.X (Math|Vector|BreakVector _returnvalue_2)) (.Y (Math|Vector|BreakVector _returnvalue_2)) 0.0))) -1.0)) -1.0) 2.7e+02)))))))))

(fn ConstructionScript)