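; Moving platform that bounces back and forth along any combination of X, Y and Z, over a set distance and speed.
; BeginPlay builds the normalized offset, then a timeline lerps the Cube's relative location, reversing after a pause at each end.
; A valid Player reference, not assigned here, is carried by setting its location on the moving axes from platform position plus its stored offset, with Animate turned off.
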(event Custom|Move
  (bind _player (Variables|Default|GetPlayer))
  (bind _returnvalue (Transformation|GetActorLocation _player))
  (bind _postiondifference (Variables|/Game/ThirdPerson/Blueprints/BP_ThirdPersonCharacter.BP_ThirdPersonCharacter_C|GetPostionDifference _player))
  (if (Variables|Default|GetDirection)
    (bind _newtrack_0 (Timeline|Timeline Play)
      (:Update
        (Transformation|SetRelativeLocation (Variables|Default|GetCube) (Math|Vector|Lerp(Vector) "0, 0, 0" (Variables|Default|GetEnd) _newtrack_0) false false)
        (if (Utilities|IsValid _player)
          (Variables|/Game/ThirdPerson/Blueprints/BP_ThirdPersonCharacter.BP_ThirdPersonCharacter_C|SetAnimate _player false)
          (Variables|Default|SetPlayerLocation "0, 0, 0")
          (if (Variables|Default|GetX_Mouvement)
            (Variables|Default|SetPlayerLocation (+ (Variables|Default|GetPlayerLocation) (Math|Vector|MakeVector (+ (.x (+ (Math|Vector|Lerp(Vector) "0, 0, 0" (Variables|Default|GetEnd) _newtrack_0) (Transformation|GetActorLocation))) (.x _postiondifference)) 0.0 0.0)))
            (else
              (Variables|Default|SetPlayerLocation (+ (Variables|Default|GetPlayerLocation) (Math|Vector|MakeVector (.x _returnvalue) 0.0 0.0)))))
          (if (Variables|Default|GetY_Mouvement)
            (Variables|Default|SetPlayerLocation (+ (Variables|Default|GetPlayerLocation) (Math|Vector|MakeVector 0.0 (+ (.y (+ (Math|Vector|Lerp(Vector) "0, 0, 0" (Variables|Default|GetEnd) _newtrack_0) (Transformation|GetActorLocation))) (.y _postiondifference)) 0.0)))
            (else
              (Variables|Default|SetPlayerLocation (+ (Variables|Default|GetPlayerLocation) (Math|Vector|MakeVector 0.0 (.y _returnvalue) 0.0)))))
          (if (Variables|Default|GetZ_Mouvement)
            (Variables|Default|SetPlayerLocation (+ (Variables|Default|GetPlayerLocation) (Math|Vector|MakeVector 0.0 0.0 (+ (.z (+ (Math|Vector|Lerp(Vector) "0, 0, 0" (Variables|Default|GetEnd) _newtrack_0) (Transformation|GetActorLocation))) (.z _postiondifference)))))
            (else
              (Variables|Default|SetPlayerLocation (+ (Variables|Default|GetPlayerLocation) (Math|Vector|MakeVector 0.0 0.0 (.z _returnvalue))))))
          (Transformation|SetActorLocation (Variables|Default|GetPlayer) (Variables|Default|GetPlayerLocation) false false)))
      (:Finished
        (Utilities|FlowControl|Delay (Math|Conversions|ToFloat(Integer) (Variables|Default|GetTimePause)))
        (if (Variables|Default|GetDirection)
          (Variables|Default|SetDirection false)
          (else
            (Variables|Default|SetDirection true)))
        (CallFunction|Move)))
    (else
      (Timeline|Timeline Reverse))))

(event EventBeginPlay
  (|CallParentFunction)
  (if (Variables|Default|GetX_Mouvement)
    (Variables|Default|SetMouvement (+ (Variables|Default|GetMouvement) "1.000000,0.000000,0.000000")))
  (if (Variables|Default|GetY_Mouvement)
    (Variables|Default|SetMouvement (+ (Variables|Default|GetMouvement) "0.000000,1.000000,0.000000")))
  (if (Variables|Default|GetZ_Mouvement)
    (Variables|Default|SetMouvement (+ (Variables|Default|GetMouvement) "0.000000,0.000000,1.000000")))
  (Variables|Default|SetMouvement (Math|Vector|Normalize (Variables|Default|GetMouvement)))
  (Variables|Default|SetEnd (* (Variables|Default|GetMouvement) (Variables|Default|GetDistance)))
  (Components|Timeline|SetPlayRate (Variables|Default|GetTimeline) (Variables|Default|GetSpeed))
  (CallFunction|Move))

(event Collision|EventActorBeginOverlap
  (params (OtherActor :type Actor%20Object%20Reference))
  (|CallParentFunction OtherActor) ; This node is disabled and will not be called.\nDrag off pins to build functionality.
)

(event EventTick
  (params (DeltaSeconds :type Float%20%28single-precision%29))
  (|CallParentFunction DeltaSeconds) ; This node is disabled and will not be called.\nDrag off pins to build functionality.
)

(fn ConstructionScript
  (|CallParentFunction))