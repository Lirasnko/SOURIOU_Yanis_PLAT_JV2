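; BP_Spawner is a spawner actor that places a single item of a configurable class above its own location.
; BeginPlay calls the Spawn event, which spawns ItemClass slightly above the actor only while the stored Item reference is invalid.
; It stores the new item and sets that item's Spawner reference to itself, linking the two in both directions.
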(event Custom|Spawn
  (if (not (Utilities|IsValid (Variables|Default|GetItem)))
    (bind _returnvalue (Game|SpawnActorfromClass (Variables|Default|GetItemClass) (Math|Transform|MakeTransform (+ (Transformation|GetActorLocation) "0.000000,0.000000,100.000000") "0, 0, 0" "1.000000,1.000000,1.000000") "Undefined" "MultiplyWithRoot" 0 0))
    (bind _output_get (Variables|Default|SetItem _returnvalue))
    (Variables|/Game/Blueprints/Item/BP_Item.BP_Item_C|SetSpawner _output_get self)))

(event EventBeginPlay
  (CallFunction|Spawn))

(event Collision|EventActorBeginOverlap
  (params (OtherActor :type Actor%20Object%20Reference)))

(event EventTick
  (params (DeltaSeconds :type Float%20%28single-precision%29)))

(fn ConstructionScript)